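; BP_FractalScreen builds a square grid of screen meshes for the 2D fractal visualizer.
; The construction script sizes each cell from the mesh bounds and adds ScreenCountXY by ScreenCountXY static mesh components edge to edge.
; Each tile gets a dynamic instance of VisualizeMaterial that receives the grid size and its own X/Y index as vector parameters.
; The event graph holds no active logic.
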(event EventBeginPlay)

(event Collision|EventActorBeginOverlap
  (params (OtherActor :type Actor%20Object%20Reference)))

(event EventTick
  (params (DeltaSeconds :type Float%20%28single-precision%29)))

(fn ConstructionScript
  (bind _screencountxy (Variables|Default|GetScreenCountXY))
  (bind _screencountxy_2 (Variables|Default|GetScreenCountXY))
  (bind _screenmesh (Variables|Default|GetScreenMesh))
  (bind _returnvalue (StaticMesh|GetBounds _screenmesh))
  (bind _returnvalue_2 (- _screencountxy 1))
  (Variables|Default|SetScreenSize (Math|Vector|MakeVector (* (.x (.boxextent _returnvalue)) 2.0) (* (.y (.boxextent _returnvalue)) 2.0) 0.0))
  (for _index (range 0 _returnvalue_2)
    (Variables|Default|SetIndexX (Math|Conversions|ToFloat(Integer) _index))
    (for _index_2 (range 0 _returnvalue_2)
      (Variables|Default|SetIndexY (Math|Conversions|ToFloat(Integer) _index_2))
      (bind _returnvalue_3 (AddComponent|AddStaticMeshComponent false (Math|Transform|MakeTransform (Math|Vector|MakeVector (* (Variables|Default|GetIndexX) (.x (Variables|Default|GetScreenSize))) (* (.y (Variables|Default|GetScreenSize)) (Variables|Default|GetIndexY)) 0.0) "0, 0, 0" "1,1,1")))
      (bind _output_get (LocalVariables|SetCurrentMeshComponent _returnvalue_3))
      (Components|StaticMesh|SetStaticMesh _output_get (Variables|Default|GetScreenMesh))
      (bind _returnvalue_4 (Rendering|Material|CreateDynamicMaterialInstance (LocalVariables|GetCurrentMeshComponent) 0 (Variables|Default|GetVisualizeMaterial) "None" :!class /Script/Engine.PrimitiveComponent))
      (Rendering|Material|SetVectorParameterValue _returnvalue_4 "ScreenCount" (Utilities|Struct|MakeLinearColor (Math|Conversions|ToFloat(Integer) _screencountxy_2) (Math|Conversions|ToFloat(Integer) _screencountxy_2) 0.0 1.0) :!class /Script/Engine.MaterialInstanceDynamic)
      (Rendering|Material|SetVectorParameterValue _returnvalue_4 "ScreenIndex" (Utilities|Struct|MakeLinearColor (Variables|Default|GetIndexX) (Variables|Default|GetIndexY) 0.0 1.0) :!class /Script/Engine.MaterialInstanceDynamic))))