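; BP_HeightMapProcessActor drives video playback and generates height and normal map render targets for the 2D fractal visualizer.
; Enter opens the media source and seeks to 1:30, while Space toggles pause; on reaching the end, playback switches to reverse.
; Every tick it draws a passthrough material into the height map target, then a height-to-normal material into the normal map target.
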(event Custom|OnEndReached_Event_0
  (bind _mediaplayah (Variables|Default|GetMediaPlayah))
  (Class|MediaPlayer|SetRate _mediaplayah -1.0)
  (Media|MediaPlayer|Play _mediaplayah :!class /Script/MediaAssets.MediaPlayer))

(event Collision|EventActorBeginOverlap
  (params (OtherActor :type Actor%20Object%20Reference)))

(event EventTick
  (params (DeltaSeconds :type Float%20%28single-precision%29))
  ;[1 1 1] Passthrough
  (Rendering|DrawMaterialtoRenderTarget "/TBRaymarcherPlugin/Fractals/2DFractalVisualizer/HeightMap_RT.HeightMap_RT" "/TBRaymarcherPlugin/Fractals/2DFractalVisualizer/M_Heighmap_Passthrough.M_Heighmap_Passthrough")
  ;[1 1 1] Get Normal Map from height map
  (Rendering|DrawMaterialtoRenderTarget "/TBRaymarcherPlugin/Fractals/2DFractalVisualizer/NormalMap_RT.NormalMap_RT" "/TBRaymarcherPlugin/Fractals/2DFractalVisualizer/M_HeightMapToNormalMap.M_HeightMapToNormalMap"))

(event Input|KeyboardEvents|SpaceBar
  (params (Key :type Key%20Structure :default "None"))
  (bind _mediaplayah (Variables|Default|GetMediaPlayah))
  (:Pressed
    (if (Class|MediaPlayer|IsPaused (Variables|Default|GetMediaPlayah))
      (Media|MediaPlayer|Play _mediaplayah :!class /Script/MediaAssets.MediaPlayer)
      (else
        (Sequencer|Player|Pause _mediaplayah)))))

(event Input|KeyboardEvents|Enter
  (params (Key :type Key%20Structure :default "None"))
  (bind _mediaplayah (Variables|Default|GetMediaPlayah))
  (:Pressed
    (bind _returnvalue (Media|MediaPlayer|OpenSource _mediaplayah (Variables|Default|GetMediaSource)))
    (if _returnvalue
      (Media|MediaPlayer|Play _mediaplayah :!class /Script/MediaAssets.MediaPlayer)
      (Media|MediaPlayer|Seek _mediaplayah (Math|Timespan|MakeTimespan 0 0 1 30 0))
      (EventDispatchers|AssignOnEndReached (Variables|Default|GetMediaPlayah) (delegate Custom|OnEndReached_Event_0))
      (else
        (Development|PrintString "Failed opening media source")))))

(fn ConstructionScript)